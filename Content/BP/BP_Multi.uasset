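; BP_Multi is a door Blueprint that opens once enough lights have been collected.
; CollectLight increments a counter and calls OpenDoor when it reaches the required amount.
; OpenDoor plays a timeline whose track lerps the static mesh's relative location downward, sinking the door out of the way.
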(event `/Game/BP/BPI_CollectLight.CollectLight`
  (`/Engine/EditorBlueprintResources/StandardMacros.IncrementInt` (`self.LightCollected`)
    (:`  `
      (if (>= (`self.LightCollected`) (`self.LightNecessary`))
        (`self.openDoor`)))))

(event `OpenDoor`
  (bind (_direction _opentrack) (`Timeline|Timeline`)
    (:`Update`
      (`SceneComponent.K2_SetRelativeLocation` (`self.StaticMeshComponent1`) (`KismetMathLibrary.VLerp` (0.0 0.0 0.0) (0.0 0.0 -400.0) _opentrack) false false))))

(fn `UserConstructionScript`)