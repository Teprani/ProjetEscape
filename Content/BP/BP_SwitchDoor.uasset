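; BP_SwitchDoor is a door that opens by sliding its mesh downward when enough switches are active.
; SwitchOn and SwitchOff events raise or lower an active pressure count and compare it with the required count.
; A timeline lerps the mesh's relative location, playing to open and reversing to close.
; SwitchOn opens only on an exact match, so exceeding the required count closes the door.
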(event `SwitchOn`
  (`/Engine/EditorBlueprintResources/StandardMacros.IncrementInt` (`self.PressureActive`)
    (:`  `
      (if (== (`self.PressureActive`) (`self.PressureNedeed`))
        (bind (_direction _opentrack) (`Timeline|Timeline` :!label _label)
          (:`Update`
            (`SceneComponent.K2_SetRelativeLocation` (`self.StaticMeshComponent1`) (`KismetMathLibrary.VLerp` (0.0 0.0 0.0) (0.0 0.0 -600.0) _opentrack) false false)))
        (else
          (goto _label :!via `Reverse`))))))

(event `SwitchOff`
  (`/Engine/EditorBlueprintResources/StandardMacros.DecrementInt` (`self.PressureActive`)
    (:`  `
      (if (< (`self.PressureActive`) (`self.PressureNedeed`))
        (goto _label :!via `Reverse`)
        (else
          (goto _label))))))

(fn `UserConstructionScript`)